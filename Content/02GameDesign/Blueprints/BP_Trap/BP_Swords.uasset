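; A sword trap projectile Blueprint that flies in a straight line and damages actors it touches.
; Tick slides the Sword component along negative local X at constant speed and destroys the actor once it exceeds MaxDistance from its origin.
; SwordCollider overlaps send a DamagePackageMessage to the overlapping actor.
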(event OnComponentBeginOverlap(SwordCollider)
  (params (OverlappedComponent :type Primitive%20Component%20Object%20Reference) (OtherActor :type Actor%20Object%20Reference) (OtherComp :type Primitive%20Component%20Object%20Reference) (OtherBodyIndex :type Integer) (bFromSweep :type Boolean) (SweepResult :type Hit%20Result%20Structure%20%28by%20ref%29))
  (Class|BPIInteraction|DamagePackage(Message) OtherActor))

(event EventTick
  (params (DeltaSeconds :type Float%20%28single-precision%29))
  (Transformation|AddLocalOffset (Variables|Default|GetSword) (Math|Vector|MakeVector (* DeltaSeconds -1.5e+02) 0.0 0.0) false false)
  (if (> (Math|Float|Absolute(Float) (.x (Variables|/Script/Engine.SceneComponent|GetRelativeLocation (Variables|Default|GetSword)))) (Variables|Default|GetMaxDistance))
    (Actor|DestroyActor)))

(fn ConstructionScript)